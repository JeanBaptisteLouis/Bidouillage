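; Energy pickup that scatters on spawn and turns into energy sent to the player when a BP_Golem overlaps it.
; On BeginPlay a timeline moves it a random horizontal distance, with a separate height curve layered on the lerp.
; An initial sphere overlap check and the collision overlap event both call SpawnSentEnergy.
; That event spawns BP_SentEnergy at StartLocation, targeting the player character, then destroys the ball.
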(event `self.ReceiveBeginPlay`
  (bind (_returnvalue_x _returnvalue_y) (`KismetMathLibrary.BreakVector` (`KismetMathLibrary.RandomUnitVector`)))
  (bind (_startlocation_x _startlocation_y) (`KismetMathLibrary.BreakVector` (`self.StartLocation`)))
  (bind (_targetlocation_x _targetlocation_y) (`KismetMathLibrary.BreakVector` (`self.TargetLocation`)))
  (for _array_element (`PrimitiveComponent.GetOverlappingActors` (`self.Sphere`) "/Game/Player/BP_Golem.BP_Golem_C")
    (cast `/Game/Player/BP_Golem` _array_element)
    (`self.SpawnSentEnergy`))
  (set `self.EndOffset` (`KismetMathLibrary.Normal` (`KismetMathLibrary.MakeVector` _returnvalue_x _returnvalue_y)))
  (set `self.StartLocation` (`self.K2_GetActorLocation`))
  (set `self.TargetLocation` (+ (`self.StartLocation`) (* (`self.EndOffset`) (`KismetMathLibrary.RandomFloatInRange` 40.0 120.0))))
  (bind (_direction _positionlerp _heightlerp) (`Timeline|Timeline`)
    (:`Update`
      (`self.K2_SetActorLocation` (+ (`KismetMathLibrary.VLerp` (`KismetMathLibrary.MakeVector` _startlocation_x _startlocation_y) (`KismetMathLibrary.MakeVector` _targetlocation_x _targetlocation_y) _positionlerp) (`KismetMathLibrary.VLerp` (0.0 0.0 0.0) (0.0 0.0 50.0) _heightlerp))))))

(event `self.Collision.OnComponentBeginOverlap`
  (params (OverlappedComponent :type "PrimitiveComponent Object Reference") (OtherActor :type "Actor Object Reference") (OtherComp :type "PrimitiveComponent Object Reference") (OtherBodyIndex :type Integer) (bFromSweep :type Boolean) (SweepResult :type "HitResult Structure (by ref)"))
  (cast `/Game/Player/BP_Golem` OtherActor)
  (`self.SpawnSentEnergy`))

(event `SpawnSentEnergy`
  (`|SpawnActorFromClass` "/Game/Energy/BP_SentEnergy.BP_SentEnergy_C" (`KismetMathLibrary.MakeTransform` (`self.StartLocation`)) "Undefined" "MultiplyWithRoot" null (`GameplayStatics.GetPlayerCharacter` 0) self true null)
  (`self.K2_DestroyActor`))

(fn `UserConstructionScript`)