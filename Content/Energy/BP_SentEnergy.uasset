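; BP_SentEnergy is an energy projectile that flies from a start actor to a targeted actor.
; A timeline lerps between both actors' live locations, adding a curve-driven height arc and a random horizontal offset to bend the path.
; On arrival it sends the target an energy message and destroys itself after a short delay.
; When ToPlayer is set, it also calls SetEnergy on the target BP_Golem.
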(event `self.ReceiveBeginPlay`
  (bind (_returnvalue_x _returnvalue_y) (`KismetMathLibrary.BreakVector` (`KismetMathLibrary.RandomUnitVector`)))
  (bind (_startoffset_x _startoffset_y) (`KismetMathLibrary.BreakVector` (`self.startOffset`)))
  (set `self.startOffset` (`KismetMathLibrary.Normal` (`KismetMathLibrary.MakeVector` _returnvalue_x _returnvalue_y)))
  (set `self.StartLocation` (`self.K2_GetActorLocation` (`self.StartActor`)))
  (set `self.EndLocation` (`self.K2_GetActorLocation` (`self.TargetedActor`)))
  (bind (_direction _alpha _alpha2 _alpha3) (`Timeline|Timeline` :!via `PlayFromStart`)
    (:`Update`
      (`|ExecutionSequence`
        (:`then_0`
          (bind _startactor (`self.StartActor`)
            (:`then`
              (set `self.StartLocation` (`self.K2_GetActorLocation` _startactor)))
            (:`else`)))
        (:`then_1`
          (bind _targetedactor (`self.TargetedActor`)
            (:`then`
              (set `self.EndLocation` (`self.K2_GetActorLocation` _targetedactor)))
            (:`else`)))
        (:`then_2`
          (`self.K2_SetActorLocation` (+ (`KismetMathLibrary.VLerp` (`self.StartLocation`) (`self.EndLocation`) _alpha) (`KismetMathLibrary.MakeVector` (* _startoffset_x 100.0 _alpha3) (* _startoffset_y 100.0 _alpha3) (* _alpha2 300.0)))))))
    (:`Finished`
      (`self.Hit`)
      (if (`self.bToPlayer`)
        (bind _asbp_golem (cast `/Game/Player/BP_Golem` (`self.TargetedActor`)))
        (`/Game/Player/BP_Golem.SetEnergy` _asbp_golem 1)))))

(event `Hit`
  (message `/Game/Elements/BPI_Interact.AddEnergy` (`self.TargetedActor`))
  (`KismetSystemLibrary.Delay` 0.5)
  (`self.K2_DestroyActor`))

(fn `UserConstructionScript`)