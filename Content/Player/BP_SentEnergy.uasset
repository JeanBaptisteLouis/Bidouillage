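; BP_SentEnergy is an energy projectile actor that travels from the player character to a targeted actor.
; On BeginPlay a timeline lerps it between both live positions, with separate curves adding height and a sideways offset in a random horizontal direction.
; When the timeline finishes, it calls AddEnergyMessage on the target, then destroys itself after a short delay.
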(event `self.ReceiveBeginPlay`
  (bind (_returnvalue_x _returnvalue_y) (`KismetMathLibrary.BreakVector` (`KismetMathLibrary.RandomUnitVector`)))
  (bind (_startoffset_x _startoffset_y) (`KismetMathLibrary.BreakVector` (`self.startOffset`)))
  (set `self.startOffset` (`KismetMathLibrary.Normal` (`KismetMathLibrary.MakeVector` _returnvalue_x _returnvalue_y)))
  (bind (_direction _alpha _alpha2 _alpha3) (`Timeline|Timeline` :!via `PlayFromStart`)
    (:`Update`
      (`self.K2_SetActorLocation` (+ (`KismetMathLibrary.VLerp` (`self.K2_GetActorLocation` (`GameplayStatics.GetPlayerCharacter` 0)) (`self.K2_GetActorLocation` (`self.TargetedActor`)) _alpha) (`KismetMathLibrary.MakeVector` (* _startoffset_x 100.0 _alpha3) (* _startoffset_y 100.0 _alpha3) (* _alpha2 300.0)))))
    (:`Finished`
      (`self.Hit`))))

(event `Hit`
  (message `/Game/Elements/BPI_Interact.AddEnergy` (`self.TargetedActor`))
  (`KismetSystemLibrary.Delay` 1.0)
  (`self.K2_DestroyActor`))

(fn `UserConstructionScript`)