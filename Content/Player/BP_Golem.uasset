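; Player golem character with orbit camera, camera-relative movement and cursor aiming on the Z=0 plane.
; A state enum drives walking, flying and a three-step lunging combo that spawns BP_GolemSpell, using timelines and gated reset windows.
; Timers drain shared energy during flight and cursor-area interaction, updating an auto-hiding energy bar.
; Tick smooths mesh rotation, computes an animation straightness factor and fades Niagara effects by speed and state.
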(event `Initialize VFX`
  (bind _mesh (`self.Mesh`))
  (`SceneComponent.K2_AttachToComponent` (`self.NS_Energy_Invoc`) _mesh "arm_L_endSocket" "SnapToTarget" "SnapToTarget" "KeepWorld" true)
  (`SceneComponent.K2_AttachToComponent` (`self.NS_Energy_Invoc_01`) _mesh "arm_R_endSocket" "SnapToTarget" "SnapToTarget" "KeepWorld" true))

(event `Initialize Variables`
  (set `self.Initial Max Speed` (`CharacterMovementComponent.MaxWalkSpeed` (`self.CharacterMovement`))))

(event `self.ReceiveBeginPlay`
  (bind _energybar_ref (`self.EnergyBar_REF`))
  (bind _asplayer_controller (cast `PlayerController` (`self.GetController`)))
  (bind _output_get (set `self.As Player Controller` _asplayer_controller))
  (`EnhancedInputSubsystemInterface.AddMappingContext` (pcsubsystem `EnhancedInputLocalPlayerSubsystem` _output_get) "/Game/Player/Inputs/IMC_Player.IMC_Player" 0 (struct))
  (`WidgetBlueprintLibrary.SetInputMode_GameAndUIEx` (`self.As Player Controller`) null "DoNotLock" false)
  (set `PlayerController.bShowMouseCursor` true (`self.As Player Controller`))
  (`self.Initialize Variables`)
  (`self.Initialize VFX`)
  (bind _asw_player_energy_bar (cast `/Game/UI/W_PlayerEnergyBar` (`WidgetComponent.GetWidget` (`self.EnergyBar`))))
  (set `self.EnergyBar_REF` _asw_player_energy_bar)
  (`self.EnergyToBarPercent`)
  (`/Game/UI/W_PlayerEnergyBar.SetEneryBarPercent` _energybar_ref)
  (`Widget.SetRenderOpacity` _energybar_ref 0.0))

(event `self.ReceiveTick`
  (params (DeltaSeconds :type "Float (single-precision)"))
  (set `self.Delta Seconds` DeltaSeconds)
  (`|ExecutionSequence`
    (:`then_0`
      (`self.UpdateCursorLocation`)
      (`self.UpdateDustOpacity`)
      (`self.UpdateSpiritModOpacity`)
      (`self.UpdateRingInvocOpacity`))
    (:`then_1`
      (switch `/Game/Player/ENUM_PlayerState` (`self.player state`)
        (:`NewEnumerator0`
          (`self.OrientMeshToMovement` :!label _label)
          (`self.UpdateAnimStraightFactor` (`self.Delta Seconds`)))
        (:`NewEnumerator1`
          (`|ExecutionSequence`
            (:`then_0`
              (goto _label))
            (:`then_1`
              (`self.CheckFlyingCondition`))))))
    (:`then_2`
      (`self.SmoothFinalMeshOrientation`))))

(event `RotateCharacterTowardCursor`
  (bind (_returnvalue_roll _returnvalue_pitch _returnvalue_yaw) (`KismetMathLibrary.BreakRotator` (`KismetMathLibrary.Conv_VectorToRotator` (- (`self.CursorLocation`) (`self.K2_GetActorLocation`)))))
  (set `self.BaseOrientation` (`KismetMathLibrary.MakeRotator` 0.0 0.0 _returnvalue_yaw)))

(event `HideEnergyBar`
  ;[0.1899 0.3958 0.1531] EnergyBar
  (`KismetSystemLibrary.K2_ClearAndInvalidateTimerHandle` (`self.EnergyBarHideTimerHandler`))
  (bind (_direction _energybaropacity) (`Timeline|Timeline` :!via `PlayFromStart` :!label _label_2)
    (:`Update`
      (`Widget.SetRenderOpacity` (`self.EnergyBar_REF`) (`KismetMathLibrary.Lerp` 0.0 1.0 _energybaropacity)))))

(event `ShowEnergyBar`
  ;[0.1899 0.3958 0.1531] EnergyBar
  (goto _label_2 :!via `ReverseFromEnd`))

(event `EnhancedInput|/Game/Player/Inputs/PlayerActions/IA_Orbit`
  (params (ActionValue :type "Float (double-precision)") (ElapsedSeconds :type "Float (double-precision)") (TriggeredSeconds :type "Float (double-precision)") (InputAction :type "InputAction Object Reference" :default "/Game/Player/Inputs/PlayerActions/IA_Orbit.IA_Orbit"))
  (:`Triggered`
    (`SceneComponent.K2_AddRelativeRotation` (`self.SpringArm`) (`KismetMathLibrary.MakeRotator` 0.0 0.0 (* ActionValue (`GameplayStatics.GetWorldDeltaSeconds`) (`self.OrbitSpeed`) -1.0)) false false)))

(event `Key|F`
  (params (Key :type "Key Structure"))
  ;[0.1899 0.3958 0.1531] EnergyBar
  (:`Pressed`
    (`self.SetEnergy` 10)))

(event `Key|G`
  (params (Key :type "Key Structure"))
  ;[0.1899 0.3958 0.1531] EnergyBar
  (:`Pressed`
    (`self.SetEnergy` -10)))

(event `EnhancedInput|/Game/Player/Inputs/PlayerActions/IA_Move`
  (params (ActionValue :type "Vector2D Structure") (ElapsedSeconds :type "Float (double-precision)") (TriggeredSeconds :type "Float (double-precision)") (InputAction :type "InputAction Object Reference" :default "/Game/Player/Inputs/PlayerActions/IA_Move.IA_Move"))
  (bind (_relativerotation_roll _relativerotation_pitch _relativerotation_yaw) (`KismetMathLibrary.BreakRotator` (`SceneComponent.RelativeRotation` (`self.SpringArm`))))
  (bind (_returnvalue_x _returnvalue_y) (`KismetMathLibrary.BreakVector` (`KismetMathLibrary.GreaterGreater_VectorRotator` (`KismetMathLibrary.MakeVector` ActionValue_X ActionValue_Y) (`KismetMathLibrary.MakeRotator` 0.0 0.0 _relativerotation_yaw))))
  (:`Triggered`
    (switch `/Game/Player/ENUM_PlayerState` (`self.player state`)
      (:`NewEnumerator0`
        _)
      (:`NewEnumerator1`
        _))
    (`self.AddMovementInput` (`KismetMathLibrary.MakeVector` _returnvalue_x _returnvalue_y))))

(event `EnhancedInput|/Game/Player/Inputs/PlayerActions/IA_Attack`
  (params (ActionValue :type Boolean) (ElapsedSeconds :type "Float (double-precision)") (TriggeredSeconds :type "Float (double-precision)") (InputAction :type "InputAction Object Reference" :default "/Game/Player/Inputs/PlayerActions/IA_Attack.IA_Attack"))
  (bind _returnvalue (`KismetMathLibrary.Normal` (- (`self.CursorLocation`) (`self.K2_GetActorLocation`))))
  (:`Triggered`
    (if (`self.canAttack`)
      (switch `/Game/Player/ENUM_PlayerState` (`self.player state`)
        (:`NewEnumerator0`
          _)
        (:`NewEnumerator1`
          (`self.CancelFlying`)))
      (set `self.player state` "NewEnumerator3")
      (`self.cancel sending`)
      (switch `int` (`self.attack_state`)
        (:`0`
          (`|ExecutionSequence`
            (:`then_0`
              (set `self.canAttack` false))
            (:`then_1`
              (set `self.attack_state` 1)
              (`self.RotateCharacterTowardCursor`)
              (`|ExecutionSequence`
                (:`then_0`
                  (bind (_direction _alpha) (`Timeline|Combo1` :!via `PlayFromStart`)
                    (:`Update`
                      (`self.AddMovementInput` (`SceneComponent.GetForwardVector` (`self.Mesh`)) _alpha))
                    (:`Finished`
                      (set `self.canAttack` true)
                      (set `self.player state` "NewEnumerator0")
                      (`|ExecutionSequence`
                        (:`then_0`
                          (goto _label_3 :!via `Open`))
                        (:`then_1`
                          (`KismetSystemLibrary.Delay` 0.5)
                          (`/Engine/EditorBlueprintResources/StandardMacros.Gate` true :!label _label_3
                            (:`Exit`
                              (set `self.attack_state` 0 :!label _label_4)
                              (if (`|EnumEquality` (`self.player state`) "NewEnumerator3")
                                (set `self.player state` "NewEnumerator0")))))))))
                (:`then_1`
                  (`self.CastSpell` 200.0 0.0 _returnvalue))))))
        (:`1`
          (`|ExecutionSequence`
            (:`then_0`
              (set `self.canAttack` false))
            (:`then_1`
              (`TimelineComponent.Stop` (`self.Combo1`))
              (set `self.attack_state` 2)
              (`self.RotateCharacterTowardCursor`)
              (`|ExecutionSequence`
                (:`then_0`
                  (goto _label_3 :!via `Close`))
                (:`then_1`
                  (bind (_direction_2 _alpha_2) (`Timeline|Combo2` :!via `PlayFromStart`)
                    (:`Update`
                      (`self.AddMovementInput` (`SceneComponent.GetForwardVector` (`self.Mesh`)) _alpha_2))
                    (:`Finished`
                      (set `self.canAttack` true)
                      (set `self.player state` "NewEnumerator0")
                      (`|ExecutionSequence`
                        (:`then_0`
                          (goto _label_5 :!via `Open`))
                        (:`then_1`
                          (`KismetSystemLibrary.Delay` 0.5)
                          (`/Engine/EditorBlueprintResources/StandardMacros.Gate` true :!label _label_5
                            (:`Exit`
                              (goto _label_4))))))))
                (:`then_2`
                  (`self.CastSpell` 300.0 30.0 _returnvalue))))))
        (:`2`
          (`|ExecutionSequence`
            (:`then_0`
              (set `self.canAttack` false))
            (:`then_1`
              (`TimelineComponent.Stop` (`self.Combo2`))
              (set `self.attack_state` 3)
              (`self.RotateCharacterTowardCursor`)
              (`|ExecutionSequence`
                (:`then_0`
                  (goto _label_5 :!via `Close`))
                (:`then_1`
                  (bind (_direction_3 _alpha_3) (`Timeline|Combo3` :!via `PlayFromStart`)
                    (:`Update`
                      (`self.AddMovementInput` (`SceneComponent.GetForwardVector` (`self.Mesh`)) _alpha_3))
                    (:`Finished`
                      (set `self.canAttack` true)
                      (set `self.player state` "NewEnumerator0")
                      (`|ExecutionSequence`
                        (:`then_0`
                          (goto _label_6 :!via `Open`))
                        (:`then_1`
                          (`KismetSystemLibrary.Delay` 0.5)
                          (`/Engine/EditorBlueprintResources/StandardMacros.Gate` true :!label _label_6
                            (:`Exit`
                              (goto _label_4))))))))
                (:`then_2`
                  (`self.CastSpell` 500.0 360.0 _returnvalue))))))))))

(event `EnhancedInput|/Game/Player/Inputs/PlayerActions/IA_Interact`
  (params (ActionValue :type Boolean) (ElapsedSeconds :type "Float (double-precision)") (TriggeredSeconds :type "Float (double-precision)") (InputAction :type "InputAction Object Reference" :default "/Game/Player/Inputs/PlayerActions/IA_Interact.IA_Interact"))
  (:`Triggered`
    (if (and ActionValue (> (`self.Energy`) 0))
      (switch `/Game/Player/ENUM_PlayerState` (`self.player state`)
        (:`NewEnumerator0`
          (bind _returnvalue (`KismetSystemLibrary.K2_SetTimerDelegate` (delegate `Interact`) 0.1 true -0.1))
          (set `self.sending` true)))
      (else
        (`KismetSystemLibrary.K2_PauseTimerHandle` _returnvalue :!label _label_7)
        (set `self.sending` false)))))

(event `cancel sending`
  (goto _label_7))

(event `Interact`
  (switch `/Game/Player/ENUM_PlayerState` (`self.player state`)
    (:`NewEnumerator0`
      (bind _outactors (`KismetSystemLibrary.SphereOverlapActors` (`self.CursorLocation`) 100.0 (`|MakeArray` "ObjectTypeQuery1" "ObjectTypeQuery2" "ObjectTypeQuery3" :!type "EObjectTypeQuery Enum")))
      (for _array_element _outactors
        (if (> (`self.Energy`) 0)
          (message `/Game/Elements/BPI_Interact.Interact` _array_element)
          (`self.SetEnergy` -1)
          (else
            (`self.cancel sending`)))))))

(event `EnhancedInput|/Game/Player/Inputs/PlayerActions/IA_Fly`
  (params (ActionValue :type Boolean) (ElapsedSeconds :type "Float (double-precision)") (TriggeredSeconds :type "Float (double-precision)") (InputAction :type "InputAction Object Reference" :default "/Game/Player/Inputs/PlayerActions/IA_Fly.IA_Fly"))
  (bind _charactermovement (`self.CharacterMovement`))
  (:`Triggered`
    (if (and ActionValue (> (`self.Energy`) 0))
      (if (and (> (`KismetMathLibrary.VSize` (`CharacterMovementComponent.GetLastUpdateVelocity` _charactermovement)) 10.0) (`NavMovementComponent.IsMovingOnGround` _charactermovement) (`|EnumEquality` (`self.player state`) "NewEnumerator0"))
        (set `CharacterMovementComponent.MaxWalkSpeed` (`self.FlySpeed`) (`self.CharacterMovement`))
        (set `self.player state` "NewEnumerator1")
        (`PrimitiveComponent.SetCollisionResponseToChannel` (`self.CapsuleComponent`) "ECC_Pawn" "ECR_Ignore")
        (bind _returnvalue (`KismetSystemLibrary.K2_SetTimerDelegate` (`|CreateDelegate` :!event `FlyConsumeEnergy`) 0.1 true))
        (set `self.FlyConsumeEnergyTimerHandler` _returnvalue))
      (else
        (set `CharacterMovementComponent.MaxWalkSpeed` (`self.Initial Max Speed`) (`self.CharacterMovement`) :!label _label_8)
        (`PrimitiveComponent.SetCollisionResponseToChannel` (`self.CapsuleComponent`) "ECC_Pawn" "ECR_Ignore")
        (set `self.player state` "NewEnumerator0")
        (`KismetSystemLibrary.K2_ClearAndInvalidateTimerHandle` (`self.FlyConsumeEnergyTimerHandler`))))))

(event `CastSpell`
  (params (radius :type "Float (double-precision)") (angle :type "Float (double-precision)") (direction :type "Vector Structure"))
  (`|SpawnActorFromClass` "/Game/Player/Combat/BP_GolemSpell.BP_GolemSpell_C" (`KismetMathLibrary.MakeTransform` (`self.K2_GetActorLocation`)) "Undefined" "MultiplyWithRoot" null radius direction 20.0 null))

(event `CancelFlying`
  (goto _label_8))

(fn `CheckFlyingCondition`
  (if (< (`KismetMathLibrary.VSize` (`CharacterMovementComponent.GetLastUpdateVelocity` (`self.CharacterMovement`))) 10.0)
    (`self.CancelFlying`)))

(fn `EnergyToBarPercent`
  (set `/Game/UI/W_PlayerEnergyBar.Percent` (/ (`self.Energy`) (`self.MaxEnergy`)) (`self.EnergyBar_REF`))
  (return))

(fn `FlyConsumeEnergy`
  (`self.SetEnergy` -2)
  (if (<= (`self.Energy`) 0)
    (`self.CancelFlying`)))

(fn `HideEnergyBarTimer`
  (if (`KismetSystemLibrary.K2_IsValidTimerHandle` (`self.EnergyBarHideTimerHandler`))
    (`KismetSystemLibrary.K2_ClearAndInvalidateTimerHandle` (`self.EnergyBarHideTimerHandler`)))
  (bind _returnvalue (`KismetSystemLibrary.K2_SetTimerDelegate` (`|CreateDelegate` :!event `HideEnergyBar`) 3.0))
  (set `self.EnergyBarHideTimerHandler` _returnvalue))

(fn `OrientMeshToMovement`
  (bind _returnvalue (`CharacterMovementComponent.GetLastUpdateVelocity` (`self.CharacterMovement`)))
  (bind (_returnvalue_roll _returnvalue_pitch _returnvalue_yaw) (`KismetMathLibrary.BreakRotator` (`KismetMathLibrary.Conv_VectorToRotator` _returnvalue)))
  (if (> (`KismetMathLibrary.VSize` _returnvalue) 10.0)
    (set `self.BaseOrientation` (`KismetMathLibrary.MakeRotator` 0.0 0.0 _returnvalue_yaw))))

(fn `SetEnergy`
  (params (EnergyToAdd :type Integer))
  (locals (EnergyResult :type Integer))
  (if (not (`KismetSystemLibrary.K2_IsValidTimerHandle` (`self.EnergyBarHideTimerHandler`)))
    (`self.ShowEnergyBar`))
  (set `local.EnergyResult` (+ EnergyToAdd (`self.Energy`)))
  (if (> (`local.EnergyResult`) (`self.MaxEnergy`))
    (set `self.Energy` (`self.MaxEnergy`))
    (elif (< (`local.EnergyResult`) 0)
      (set `self.Energy` 0)
      (else
        (set `self.Energy` (`local.EnergyResult`)))))
  (`self.EnergyToBarPercent`)
  (`/Game/UI/W_PlayerEnergyBar.SetEneryBarPercent` (`self.EnergyBar_REF`))
  (`self.HideEnergyBarTimer`))

(fn `SmoothFinalMeshOrientation`
  (bind _mesh (`self.Mesh`))
  (`SceneComponent.K2_SetWorldRotation` _mesh (`KismetMathLibrary.RInterpTo` (`SceneComponent.K2_GetComponentRotation` _mesh) (`self.BaseOrientation`) (`self.Delta Seconds`) 10.0) false false))

(fn `UpdateAnimStraightFactor`
  (params (DeltaTime :type "Float (single-precision)"))
  (bind _charactermovement (`self.CharacterMovement`))
  (bind _returnvalue (`CharacterMovementComponent.GetLastUpdateVelocity` _charactermovement))
  (bind _maxwalkspeed (`CharacterMovementComponent.MaxWalkSpeed` _charactermovement))
  (set `self.PreviousVelocity` (`KismetMathLibrary.VInterpTo` (`self.PreviousVelocity`) _returnvalue DeltaTime 3.0))
  (set `self.Straight` (`KismetMathLibrary.FInterpTo` (`self.Straight`) (* (`KismetMathLibrary.FClamp` (`KismetMathLibrary.Dot_VectorVector` (/ _returnvalue _maxwalkspeed) (/ (`self.PreviousVelocity`) _maxwalkspeed)) -1.0) (== (`self.attack_state`) 0)) DeltaTime 3.0)))

(fn `UpdateCursorLocation`
  (bind _returnvalue (`SceneComponent.K2_GetComponentLocation` (`self.Camera`)))
  (set `self.CursorLocation` (`.Intersection` (`KismetMathLibrary.LinePlaneIntersection` _returnvalue (+ _returnvalue (* (`.WorldDirection` (`PlayerController.DeprojectMousePositionToWorld` (`GameplayStatics.GetPlayerController` 0))) 10000.0)) (`KismetMathLibrary.MakePlaneFromPointAndNormal` (0.0 0.0 0.0) (0.0 0.0 1.0)))))
  (`KismetSystemLibrary.DrawDebugCircle` (+ (`self.CursorLocation`) (0.0 0.0 5.0)) 100.0 128 (struct :`G` 1.0 :`B` 0.990615 :`A` 1.0) 0.0 5.0 (1.0 0.0 0.0) (0.0 1.0 0.0)))

(fn `UpdateDustOpacity`
  (bind _charactermovement (`self.CharacterMovement`))
  (`FXSystemComponent.SetFloatParameter` (`self.NS_Smoke_Wind`) "Opacity" (- 1.0 (/ (`KismetMathLibrary.VSize` (`CharacterMovementComponent.GetLastUpdateVelocity` _charactermovement)) (`CharacterMovementComponent.MaxWalkSpeed` _charactermovement)))))

(fn `UpdateRingInvocOpacity`
  (bind _output_get (set `self.RingInvocFXOpacity` (`KismetMathLibrary.FInterpTo` (`self.RingInvocFXOpacity`) (`KismetMathLibrary.Conv_BoolToDouble` (`self.sending`)) (`self.Delta Seconds`) 10.0)))
  (`FXSystemComponent.SetFloatParameter` (`self.NS_Energy_Invoc_01`) "Opacity" _output_get)
  (`FXSystemComponent.SetFloatParameter` (`self.NS_Energy_Invoc`) "Opacity" _output_get))

(fn `UpdateSpiritModOpacity`
  (bind _charactermovement (`self.CharacterMovement`))
  (bind _output_get (set `self.FluingFXOpacity` (`KismetMathLibrary.FInterpTo` (`self.FluingFXOpacity`) (* (/ (`KismetMathLibrary.VSize` (`CharacterMovementComponent.GetLastUpdateVelocity` _charactermovement)) (`CharacterMovementComponent.MaxWalkSpeed` _charactermovement)) (`|EnumEquality` (`self.player state`) "NewEnumerator1")) (`self.Delta Seconds`) 10.0)))
  (`FXSystemComponent.SetFloatParameter` (`self.NS_Spirit_Mod`) "Opacity" _output_get))

(fn `UserConstructionScript`)