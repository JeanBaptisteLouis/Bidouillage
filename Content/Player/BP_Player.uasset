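; Player character with an orbitable camera, a flying mode and mouse-aimed interaction.
; Enhanced Input drives camera-relative movement, spring arm yaw, and flying, which changes walk speed and a Niagara rate.
; Tick projects the mouse onto the Z=0 plane with a debug circle, smooths mesh yaw toward velocity and updates an animation straightness factor.
; Holding interact while walking repeatedly sphere-overlaps at the cursor and sends InteractMessage to hit actors.
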(event `self.ReceiveBeginPlay`
  (bind _asplayer_controller (cast `PlayerController` (`self.GetController`)))
  (bind _output_get (set `self.As Player Controller` _asplayer_controller))
  (`EnhancedInputSubsystemInterface.AddMappingContext` (pcsubsystem `EnhancedInputLocalPlayerSubsystem` _output_get) "/Game/Player/Inputs/IMC_Player.IMC_Player" 0 (struct))
  (`WidgetBlueprintLibrary.SetInputMode_GameAndUIEx` (`self.As Player Controller`) null "DoNotLock" false)
  (set `PlayerController.bShowMouseCursor` true (`self.As Player Controller`))
  (set `self.Initial Fly Speed` (`self.FlySpeed`))
  (set `self.Initial Max Speed` (`CharacterMovementComponent.MaxWalkSpeed` (`self.CharacterMovement`))))

(event `self.ReceiveTick`
  (params (DeltaSeconds :type "Float (single-precision)"))
  (bind _output_get (set `self.Delta Seconds` DeltaSeconds))
  (`self.UpdateAnimStraightFactor` _output_get)
  (`self.UpdateCursorLocation`)
  (`self.OrientMesh`)
  (`KismetSystemLibrary.DrawDebugCircle` (+ (`self.CursorLocation`) (0.0 0.0 5.0)) 100.0 128 (struct :`G` 1.0 :`B` 0.990615 :`A` 1.0) 0.0 5.0 (1.0 0.0 0.0) (0.0 1.0 0.0)))

(event `EnhancedInput|/Game/Player/Inputs/PlayerActions/IA_Move`
  (params (ActionValue :type "Vector2D Structure") (ElapsedSeconds :type "Float (double-precision)") (TriggeredSeconds :type "Float (double-precision)") (InputAction :type "InputAction Object Reference" :default "/Game/Player/Inputs/PlayerActions/IA_Move.IA_Move"))
  (bind (_relativerotation_roll _relativerotation_pitch _relativerotation_yaw) (`KismetMathLibrary.BreakRotator` (`SceneComponent.RelativeRotation` (`self.SpringArm`))))
  (bind (_returnvalue_x _returnvalue_y) (`KismetMathLibrary.BreakVector` (`KismetMathLibrary.GreaterGreater_VectorRotator` (`KismetMathLibrary.MakeVector` ActionValue_X ActionValue_Y) (`KismetMathLibrary.MakeRotator` 0.0 0.0 _relativerotation_yaw))))
  (:`Triggered`
    (`self.AddMovementInput` (`KismetMathLibrary.MakeVector` _returnvalue_x _returnvalue_y))))

(event `EnhancedInput|/Game/Player/Inputs/PlayerActions/IA_Orbit`
  (params (ActionValue :type "Float (double-precision)") (ElapsedSeconds :type "Float (double-precision)") (TriggeredSeconds :type "Float (double-precision)") (InputAction :type "InputAction Object Reference" :default "/Game/Player/Inputs/PlayerActions/IA_Orbit.IA_Orbit"))
  (:`Triggered`
    (`SceneComponent.K2_AddRelativeRotation` (`self.SpringArm`) (`KismetMathLibrary.MakeRotator` 0.0 0.0 (* ActionValue (`GameplayStatics.GetWorldDeltaSeconds`) (`self.OrbitSpeed`))) false false)))

(event `EnhancedInput|/Game/Player/Inputs/PlayerActions/IA_Fly`
  (params (ActionValue :type Boolean) (ElapsedSeconds :type "Float (double-precision)") (TriggeredSeconds :type "Float (double-precision)") (InputAction :type "InputAction Object Reference" :default "/Game/Player/Inputs/PlayerActions/IA_Fly.IA_Fly"))
  (:`Triggered`
    (if ActionValue
      (if (`NavMovementComponent.IsMovingOnGround` (`self.CharacterMovement`))
        (set `CharacterMovementComponent.MaxWalkSpeed` (`self.FlySpeed`) (`self.CharacterMovement`))
        (set `self.State` "NewEnumerator1")
        (`FXSystemComponent.SetFloatParameter` (`self.N_Flying`) "rate" (select `/Game/Player/ENUM_PlayerState` (`self.State`) :`NewEnumerator1` 10.0 :!type "Float (single-precision)") :!label _label))
      (else
        (set `CharacterMovementComponent.MaxWalkSpeed` (`self.Initial Max Speed`) (`self.CharacterMovement`))
        (set `self.State` "NewEnumerator0")
        (goto _label)))))

(event `EnhancedInput|/Game/Player/Inputs/PlayerActions/IA_Interact`
  (params (ActionValue :type Boolean) (ElapsedSeconds :type "Float (double-precision)") (TriggeredSeconds :type "Float (double-precision)") (InputAction :type "InputAction Object Reference" :default "/Game/Player/Inputs/PlayerActions/IA_Interact.IA_Interact"))
  (:`Triggered`
    (if ActionValue
      (bind _returnvalue (`KismetSystemLibrary.K2_SetTimerDelegate` (delegate `Interact`) 0.1 true -0.1))
      (else
        (`KismetSystemLibrary.K2_PauseTimerHandle` _returnvalue)))))

(event `Interact`
  (switch `/Game/Player/ENUM_PlayerState` (`self.State`)
    (:`NewEnumerator0`
      (bind _outactors (`KismetSystemLibrary.SphereOverlapActors` (`self.CursorLocation`) 100.0 (`|MakeArray` "ObjectTypeQuery1" "ObjectTypeQuery2" "ObjectTypeQuery3" :!type "EObjectTypeQuery Enum")))
      (for _array_element _outactors
        (message `/Game/Elements/BPI_Interact.Interact` _array_element)))))

(fn `OrientMesh`
  (bind _charactermovement (`self.CharacterMovement`))
  (bind _mesh (`self.Mesh`))
  (bind _returnvalue (`CharacterMovementComponent.GetLastUpdateVelocity` _charactermovement))
  (bind (_returnvalue_roll _returnvalue_pitch _returnvalue_yaw) (`KismetMathLibrary.BreakRotator` (`SceneComponent.K2_GetComponentRotation` _mesh)))
  (bind (_returnvalue_roll_2 _returnvalue_pitch_2 _returnvalue_yaw_2) (`KismetMathLibrary.BreakRotator` (`KismetMathLibrary.Conv_VectorToRotator` _returnvalue)))
  (bind _returnvalue_2 (`KismetMathLibrary.VSize` _returnvalue))
  (if (> _returnvalue_2 0.1)
    (`SceneComponent.K2_SetWorldRotation` _mesh (`KismetMathLibrary.RInterpTo` (`KismetMathLibrary.MakeRotator` 0.0 0.0 _returnvalue_yaw) (`KismetMathLibrary.MakeRotator` 0.0 0.0 _returnvalue_yaw_2) (`self.Delta Seconds`) (* (/ _returnvalue_2 (`CharacterMovementComponent.MaxWalkSpeed` _charactermovement)) (`self.MeshRotSpeed`))) false false)))

(fn `UpdateAnimStraightFactor`
  (params (DeltaTime :type "Float (single-precision)"))
  (bind _charactermovement (`self.CharacterMovement`))
  (bind _returnvalue (`CharacterMovementComponent.GetLastUpdateVelocity` _charactermovement))
  (bind _maxwalkspeed (`CharacterMovementComponent.MaxWalkSpeed` _charactermovement))
  (set `self.PreviousVelocity` (`KismetMathLibrary.VInterpTo` (`self.PreviousVelocity`) _returnvalue DeltaTime 3.0))
  (set `self.Straight` (`KismetMathLibrary.FInterpTo` (`self.Straight`) (`KismetMathLibrary.FClamp` (`KismetMathLibrary.Dot_VectorVector` (/ _returnvalue _maxwalkspeed) (/ (`self.PreviousVelocity`) _maxwalkspeed)) -1.0) DeltaTime 3.0)))

(fn `UpdateCursorLocation`
  (bind _returnvalue (`SceneComponent.K2_GetComponentLocation` (`self.Camera`)))
  (set `self.CursorLocation` (`.Intersection` (`KismetMathLibrary.LinePlaneIntersection` _returnvalue (+ _returnvalue (* (`.WorldDirection` (`PlayerController.DeprojectMousePositionToWorld` (`GameplayStatics.GetPlayerController` 0))) 10000.0)) (`KismetMathLibrary.MakePlaneFromPointAndNormal` (0.0 0.0 0.0) (0.0 0.0 1.0))))))

(fn `UserConstructionScript`)