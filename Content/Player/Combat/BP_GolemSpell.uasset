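; BP_GolemSpell is a short-lived slash attack actor that sends a damaging wave out along Direction.
; On BeginPlay it picks a Niagara slash effect by Type and rotates it to Direction's yaw with a fixed tilt.
; A timeline moves the effect forward, drives its life parameter and grows a Pawn sphere overlap in step.
; Overlapped pawns receive damage through CHealthSystem on every update, and the actor destroys itself when the timeline finishes.
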(event `self.ReceiveBeginPlay`
  (bind (_returnvalue_roll _returnvalue_pitch _returnvalue_yaw) (`KismetMathLibrary.BreakRotator` (`KismetMathLibrary.Conv_VectorToRotator` (`self.direction`))))
  (`|ExecutionSequence`
    (:`then_0`
      (`NiagaraComponent.SetAsset` (`self.NS_Slash_01`) (select `/Game/Player/Combat/ENUM_SpellType` (`self.type`) :`NewEnumerator0` "/Game/VFX/NS/NS_Slash_First.NS_Slash_First" :`NewEnumerator1` "/Game/VFX/NS/NS_Slash_Secode.NS_Slash_Secode" :`NewEnumerator2` "/Game/VFX/NS/NS_Slash_First.NS_Slash_First" :!type "NiagaraSystem Object Reference") true))
    (:`then_1`
      (`SceneComponent.K2_SetWorldRotation` (`self.NS_Slash_01`) (`KismetMathLibrary.ComposeRotators` (`KismetMathLibrary.MakeRotator` 0.0 0.0 _returnvalue_yaw) (struct :`Yaw` 85.0)) false false)
      (bind (_direction _alpha) (`Timeline|Timeline` :!via `PlayFromStart`)
        (:`Update`
          (bind _returnvalue (* (`self.direction`) _alpha 300.0))
          (bind _outactors (`KismetSystemLibrary.SphereOverlapActors` (+ (`self.K2_GetActorLocation`) _returnvalue) (* _alpha (`self.radius`)) (`|MakeArray` "ObjectTypeQuery3" :!type "EObjectTypeQuery Enum")))
          (`/Game/Elements/C_HealthSystem.FCT_DoDamage` (`self.C_HealthSystem`) _outactors (`self.damage`))
          (`FXSystemComponent.SetFloatParameter` (`self.NS_Slash_01`) "life" _alpha)
          (`SceneComponent.K2_SetRelativeLocation` (`self.NS_Slash_01`) _returnvalue false false))
        (:`Finished`
          (`self.K2_DestroyActor`))))))

(fn `UserConstructionScript`)