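; BP_Reader is an actor that samples the RT_Map render target at its own world position and changes its mesh to reflect what it reads.
; Each Tick, it converts its location to UVs using the worldRes scalar from MPC_Global, centered on 0.5.
; It reads that raw pixel and sets its Sphere component to a sphere mesh when red is below green, otherwise to a cube.
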(event `self.ReceiveTick`
  (params (DeltaSeconds :type "Float (single-precision)"))
  (bind _sphere (`self.Sphere`))
  (bind _returnvalue (`KismetMaterialLibrary.GetScalarParameterValue` "/Game/MPC_Global.MPC_Global" "worldRes"))
  (bind _returnvalue_2 (`KismetRenderingLibrary.ReadRenderTargetRawUV` "/Game/RT/RT_Map.RT_Map" (.x (+ (/ (`self.K2_GetActorLocation`) _returnvalue) (0.5 0.5 0.0))) (.y (+ (/ (`self.K2_GetActorLocation`) _returnvalue) (0.5 0.5 0.0))) false))
  (bind (_r _g) (`KismetMathLibrary.BreakColor` _returnvalue_2))
  (if (< _r _g)
    (`StaticMeshComponent.SetStaticMesh` _sphere "/Engine/EngineMeshes/Sphere.Sphere")
    (else
      (`StaticMeshComponent.SetStaticMesh` _sphere "/Engine/BasicShapes/Cube.Cube")))
  (`KismetSystemLibrary.PrintString` (`KismetStringLibrary.Conv_DoubleToString` _r) :!enabledstate Disabled))

(fn `UserConstructionScript`)