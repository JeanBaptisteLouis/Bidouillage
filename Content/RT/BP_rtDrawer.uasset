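; BP_rtDrawer is an actor that paints its location into the shared RT_Map render target every tick and on construction.
; It draws a dynamic M_Draw material instance fed by location, Side, Grow, Power and a fixed size.
; Only the first drawer returned by GetAllActorsOfClass clears the target to red before drawing, so multiple drawers can composite into one map.
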(event `Draw`
  (bind _drawmt (`self.DrawMT`))
  (`|ExecutionSequence`
    (:`then_0`
      (bind _outactors (`GameplayStatics.GetAllActorsOfClass` "BP_rtDrawer_C"))
      (if (== (`|GetArrayItem` _outactors) self)
        (`KismetRenderingLibrary.ClearRenderTarget2D` "/Game/RT/RT_Map.RT_Map" (struct :`R` 1.0 :`A` 1.0))))
    (:`then_1`
      (`MaterialInstanceDynamic.SetScalarParameterValue` _drawmt "size" 0.1)
      (`MaterialInstanceDynamic.SetVectorParameterValue` _drawmt "offset" (`KismetMathLibrary.Conv_VectorToLinearColor` (`self.K2_GetActorLocation`)))
      (`MaterialInstanceDynamic.SetScalarParameterValue` _drawmt "Side" (`KismetMathLibrary.Conv_BoolToDouble` (`self.side`)))
      (`MaterialInstanceDynamic.SetScalarParameterValue` _drawmt "grow" (`KismetMathLibrary.Conv_BoolToDouble` (`self.grow`)))
      (`MaterialInstanceDynamic.SetScalarParameterValue` _drawmt "power" (`self.power`))
      (`KismetRenderingLibrary.DrawMaterialToRenderTarget` "/Game/RT/RT_Map.RT_Map" (`self.DrawMT`)))))

(event `self.ReceiveTick`
  (params (DeltaSeconds :type "Float (single-precision)"))
  (`self.Draw`))

(fn `UserConstructionScript`
  (bind _returnvalue (`KismetMaterialLibrary.CreateDynamicMaterialInstance` "/Game/RT/M_Draw.M_Draw"))
  (set `self.DrawMT` _returnvalue)
  (`self.Draw`))