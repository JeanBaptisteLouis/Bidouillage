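; Actor component that shows an area effect on its owner's mesh through an overlay material.
; On BeginPlay it gets the mesh from the owner with an interface message and assigns a dynamic instance of M_AreaActor as its overlay.
; SwitchArea plays or reverses a component timeline based on its boolean, with updates writing that flag to the material's area parameter and the timeline's curve to opacity.
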(event `self.ReceiveBeginPlay`
  (`ComponentTimelineLibrary.InitializeComponentTimelines` null)
  (bind _mesh (message `/Game/Elements/BPI_AreaSystem.getMesh` (`self.GetOwner`)))
  (bind _returnvalue (`KismetMaterialLibrary.CreateDynamicMaterialInstance` "/Game/AreaSystem/M_AreaActor.M_AreaActor"))
  (bind _output_get (set `self.mat` _returnvalue))
  (`MeshComponent.SetOverlayMaterial` _mesh _output_get))

(event `SwitchArea`
  (params (inArea :type Boolean))
  (if inArea
    (bind (_direction _opacity) (`|ComponentTimeline` 0.0 :!label _label)
      (:`Update`
        (`MaterialInstanceDynamic.SetScalarParameterValue` (`self.mat`) "area" (`KismetMathLibrary.Conv_BoolToDouble` inArea))
        (`MaterialInstanceDynamic.SetScalarParameterValue` (`self.mat`) "opacity" _opacity)))
    (else
      (goto _label :!via `Reverse`))))