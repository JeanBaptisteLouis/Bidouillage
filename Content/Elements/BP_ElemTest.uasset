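; Test element actor that takes in energy from the player and expands its area of effect.
; Interact spawns a BP_SentEnergy actor at the player's location, targeted at this actor.
; AddEnergy enlarges the ACArea size and resizes the AreaEffect sphere radius to slightly less than that size.
; Each energy gain also restarts a timeline that animates the Sphere's scale as a feedback pulse.
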(event `/Game/Elements/BPI_Interact.Interact`
  (bind _returnvalue (`GameplayStatics.GetPlayerCharacter` 0))
  (`|SpawnActorFromClass` "/Game/Player/BP_SentEnergy.BP_SentEnergy_C" (`KismetMathLibrary.MakeTransform` (`self.K2_GetActorLocation` _returnvalue)) "Undefined" "MultiplyWithRoot" null self _returnvalue null))

(event `/Game/Elements/BPI_Interact.AddEnergy`
  (bind _ac_area (`self.AC_Area`))
  (bind _output_get (set `/Game/AreaSystem/AC_Area.size` (+ (`/Game/AreaSystem/AC_Area.size` _ac_area) 100.0) _ac_area))
  (`SphereComponent.SetSphereRadius` (`self.area effect`) (* _output_get 0.9) true)
  (bind (_direction _alpha) (`Timeline|Timeline` :!via `PlayFromStart`)
    (:`Update`
      (`SceneComponent.SetRelativeScale3D` (`self.Sphere`) (`KismetMathLibrary.Conv_DoubleToVector` (- (+ 0.5 1.0) (* 0.5 _alpha)))))))

(fn `UserConstructionScript`)