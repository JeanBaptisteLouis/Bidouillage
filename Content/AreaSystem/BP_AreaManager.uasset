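; Area manager actor that rebuilds a map of Good, Evil and Neutral area influence in the RT_Map render target.
; Every Tick it clears the target, then loops over the area components registered in GI_Main.
; Each component's size, owner location, side and power feed one reused M_Draw dynamic material, drawn into the target once per area.
; Evil and Neutral pass the same side value to the material.
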(event `self.ReceiveBeginPlay`
  (bind _asgi_main (cast `/Game/GI_Main` (`GameplayStatics.GetGameInstance`)))
  (set `self.As GI Main` _asgi_main)
  (bind _returnvalue (`KismetMaterialLibrary.CreateDynamicMaterialInstance` "/Game/RT/M_Draw.M_Draw"))
  (set `self.DrawMT` _returnvalue))

(event `self.ReceiveTick`
  (params (DeltaSeconds :type "Float (single-precision)"))
  (bind _drawmt (`self.DrawMT`))
  (`KismetRenderingLibrary.ClearRenderTarget2D` "/Game/RT/RT_Map.RT_Map" (struct :`R` 1.0 :`A` 1.0))
  (for _array_element (`/Game/GI_Main.area_components` (`self.As GI Main`))
    (`MaterialInstanceDynamic.SetScalarParameterValue` _drawmt "size" (`/Game/AreaSystem/AC_Area.size` _array_element))
    (`MaterialInstanceDynamic.SetVectorParameterValue` _drawmt "offset" (`KismetMathLibrary.Conv_VectorToLinearColor` (`self.K2_GetActorLocation` (`ActorComponent.GetOwner` _array_element))))
    (`MaterialInstanceDynamic.SetScalarParameterValue` _drawmt "Side" (select `/Game/AreaSystem/Enum_AreaState` (`/Game/AreaSystem/AC_Area.side` _array_element) :`NewEnumerator0` 1.0 :!type "Float (single-precision)"))
    (`MaterialInstanceDynamic.SetScalarParameterValue` _drawmt "power" (`/Game/AreaSystem/AC_Area.power` _array_element))
    (`KismetRenderingLibrary.DrawMaterialToRenderTarget` "/Game/RT/RT_Map.RT_Map" (`self.DrawMT`))))

(fn `UserConstructionScript`)