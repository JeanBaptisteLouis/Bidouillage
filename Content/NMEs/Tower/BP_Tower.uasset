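; BP_Tower is an enemy tower that periodically spawns BP_FlyingNME minions and triggers its energy-giver component.
; Two looping timers drive it, one calling StartGiveEnergy and one spawning an enemy at a random offset around and above the tower, passing it the tower's location.
; Each spawn increments an enemy count, which Tick checks to pause or resume the spawn timer at a fixed cap.
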(event `CustomEvent`
  (`/Game/Components/C_EnergyGiver.StartGiveEnergy` (`self.C_EnergyGiver`)))

(event `self.ReceiveBeginPlay`
  (bind _returnvalue (`KismetSystemLibrary.K2_SetTimerDelegate` (delegate `SpawnEnemy`) 5.0 true))
  (set `self.EnemySpawnTimerHandler` _returnvalue)
  (`KismetSystemLibrary.K2_SetTimerDelegate` (delegate `CustomEvent`) 5.0 true))

(event `self.ReceiveTick`
  (params (DeltaSeconds :type "Float (single-precision)"))
  ;[1 1 1] Would be better if checked when a minion die to unpause spawn timer handler and to pause it we would check right after the spawn
  (`self.CheckTowerEnemies`))

(event `CheckTowerEnemies`
  ;[1 1 1] Would be better if checked when a minion die to unpause spawn timer handler and to pause it we would check right after the spawn
  (if (>= (`self.TowerEnemiesCount`) 20)
    (`KismetSystemLibrary.K2_PauseTimerHandle` (`self.EnemySpawnTimerHandler`))
    (elif (`KismetSystemLibrary.K2_IsTimerPausedHandle` (`self.EnemySpawnTimerHandler`))
      (`KismetSystemLibrary.K2_UnPauseTimerHandle` (`self.EnemySpawnTimerHandler`)))))

(event `SpawnEnemy`
  (bind (_returnvalue_x _returnvalue_y) (`KismetMathLibrary.BreakVector` (`KismetMathLibrary.RandomUnitVector`)))
  (`|SpawnActorFromClass` "/Game/NMEs/BP_FlyingNME.BP_FlyingNME_C" (`KismetMathLibrary.MakeTransform` (+ (`self.K2_GetActorLocation`) (* (`KismetMathLibrary.Normal` (`KismetMathLibrary.MakeVector` _returnvalue_x _returnvalue_y)) 200.0) (`KismetMathLibrary.MakeVector` 0.0 0.0 (`KismetMathLibrary.RandomFloatInRange` 50.0 150.0)))) "AdjustIfPossibleButDontSpawnIfColliding" "MultiplyWithRoot" null false 0.5 false 5 0 (+ (`self.K2_GetActorLocation`) (0.0 0.0 50.0)) null)
  (bind _result (`/Engine/EditorBlueprintResources/StandardMacros.IncrementInt` (`self.TowerEnemiesCount`))
    (:`  `
      (`KismetSystemLibrary.PrintString` (`KismetStringLibrary.Conv_IntToString` _result)))))

(fn `UserConstructionScript`)