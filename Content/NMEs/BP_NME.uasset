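; BP_NME is an actor that chases the player every tick while steering around nearby obstacles.
; It sweeps short, debug-drawn Visibility line traces in a horizontal ring, summing push-away vectors from hits, weighted by closeness.
; That avoidance sum is blended with the normalized direction to the player, renormalized and fed to FloatingPawnMovement as movement input.
; The loop's inclusive end index likely repeats the first trace direction, double-counting hits there.
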(event `self.ReceiveTick`
  (params (DeltaSeconds :type "Float (single-precision)"))
  (bind _returnvalue (`self.K2_GetActorLocation`))
  (`|ExecutionSequence`
    (:`then_0`
      (set `self.DirectionVector` (`KismetMathLibrary.Normal` (- (`self.K2_GetActorLocation` (`GameplayStatics.GetPlayerCharacter` 0)) (`self.K2_GetActorLocation`))))
      (set `self.AvoidanceVector` (0.0 0.0 0.0))
      (for _index (range (+ 8 1))
        (bind (_outhit _returnvalue_2) (`KismetSystemLibrary.LineTraceSingle` :`Start` _returnvalue :`End` (+ _returnvalue (`KismetMathLibrary.RotateAngleAxis` (`KismetMathLibrary.MakeVector` 100.0) (* (/ 360.0 (`KismetMathLibrary.Conv_IntToDouble` 8)) _index) (0.0 0.0 1.0))) :`TraceChannel` "TraceTypeQuery1" :`DrawDebugType` "ForOneFrame"))
        (if _returnvalue_2
          (bind (_bblockinghit _binitialoverlap _time _distance _location) (`GameplayStatics.BreakHitResult` _outhit))
          (set `self.AvoidanceVector` (+ (`self.AvoidanceVector`) (* (- (`self.K2_GetActorLocation`) _location) (/ (- 100.0 _distance) 100.0))))))
      (set `self.DirectionVector` (`KismetMathLibrary.Normal` (+ (`self.AvoidanceVector`) (`self.DirectionVector`)))))
    (:`then_1`
      (`PawnMovementComponent.AddInputVector` (`self.FloatingPawnMovement`) (`self.DirectionVector`) false))))

(fn `UserConstructionScript`)