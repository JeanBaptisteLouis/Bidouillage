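; Flying enemy pawn that sends an Awake event to its StateTree when the player comes within range.
; GoToPlayer restarts GoTo, which async-finds a CPathVolume path and steers node to node, setting the input vector that Move feeds to FlyingMovementComponent.
; Periodic path rechecks use velocity alignment and visibility traces to skip nodes.
; DestroyMe disables collision and animates emissive and scale before destroying the actor.
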(event `self.ReceiveTick`
  (params (DeltaSeconds :type "Float (single-precision)"))
  (bind _returnvalue (`GameplayStatics.GetPlayerCharacter` 0))
  (`/Engine/EditorBlueprintResources/StandardMacros.IsValid` _returnvalue
    (:`Is Valid`
      (set `self.NME_Location` (`self.K2_GetActorLocation`))
      (if (< (`KismetMathLibrary.Vector_Distance` (`self.K2_GetActorLocation` _returnvalue) (`self.K2_GetActorLocation`)) 1000.0)
        (`/Engine/EditorBlueprintResources/StandardMacros.DoOnce` false
          (:`Completed`
            (`self.wake up`)))))))

(event `wake up`
  (`StateTreeComponent.SendStateTreeEvent` (`self.StateTree`) (make `StateTreeEvent` (struct :`TagName` "awake")))
  (set `self.Awake` true))

(event `GoToPlayer`
  (params (Destination :type "Vector Structure"))
  (bind _output_get (set `self.Destination` Destination))
  (`|ExecutionSequence`
    (:`then_0`
      (goto _label :!via `Interupt`))
    (:`then_1`
      (`self.GoTo` _output_get :!label _label
        (:`Success`
          _)
        (:`Failed`
          _))
      (set `self.CurrentInputVector` (`self.Destination`))
      (if (`self.DestroyAfterReachingDestination`)
        (`self.DestroyMe`)))))

(event `Move`
  (`PawnMovementComponent.AddInputVector` (`self.FlyingMovementComponent`) (`self.CurrentInputVector`) false)
  (set `self.NME_Location` (`self.K2_GetActorLocation`)))

(event `DestroyMe`
  ;[1 1 1] Animating death and destroying actor
  (`PrimitiveComponent.SetCollisionEnabled` (`self.RootMesh`) "NoCollision")
  (`PrimitiveComponent.SetCollisionEnabled` (`self.Head`) "NoCollision")
  (bind _returnvalue (`PrimitiveComponent.CreateDynamicMaterialInstance` (`self.RootMesh`) 0 null "None"))
  (bind _output_get (set `self.MaterialInst` _returnvalue))
  (`PrimitiveComponent.SetMaterial` (`self.Head`) 0 _output_get)
  (`PrimitiveComponent.SetMaterial` (`self.RootMesh`) 0 _output_get)
  (bind (_direction _emissive _scale) (`Timeline|DestroyingTimeline`)
    (:`Update`
      (`MaterialInstanceDynamic.SetScalarParameterValue` (`self.MaterialInst`) "Emissive Intensity" _emissive)
      (`self.SetActorScale3D` (`KismetMathLibrary.Conv_DoubleToVector` _scale)))
    (:`Finished`
      (`self.K2_DestroyActor`))))

(fn `DrawPath`
  (if (and (`self.DrawDebugPath`) (`KismetSystemLibrary.IsValid` (`self.VolumeRef`)))
    (`CPathVolume.DrawDebugPath` (`self.VolumeRef`) (`self.PathBuffer`) 0.2 true (`self.DebugPathColor`))))

(fn `GetDotToNode`
  (params (Node :type "CPathNode Structure"))
  (returns (Dot :type "Float (double-precision)"))
  (return (`KismetMathLibrary.Dot_VectorVector` (`KismetMathLibrary.Normal` (`MovementComponent.Velocity` (`self.FlyingMovementComponent`))) (`KismetMathLibrary.Normal` (- (`.WorldLocation` (break `CPathNode` Node)) (`self.K2_GetActorLocation`))))))

(fn `GetNextOptimalNode`
  (params (CurrentNodeIndex :type Integer))
  (returns (BestNodeIndex :type Integer))
  (locals (BestIndex :type Integer) (BestDot :type "Float (double-precision)") (WasHit :type Boolean) (CurrDot :type "Float (double-precision)"))
  (bind _output (`|GetArrayItem` (`self.PathBuffer`) (+ (`local.BestIndex`) 1)))
  (set `local.BestIndex` CurrentNodeIndex)
  (set `local.BestDot` (`self.GetDotToNode` (`|GetArrayItem` (`self.PathBuffer`) CurrentNodeIndex)))
  (while (and (not (`local.WasHit`)) (< (`local.BestIndex`) (- (`KismetArrayLibrary.Array_Length` (`self.PathBuffer`)) 1)))
    (bind _output_get (set `local.CurrDot` (`self.GetDotToNode` _output)))
    (if (> _output_get (`local.BestDot`))
      (bind (_outhit _returnvalue) (`KismetSystemLibrary.LineTraceSingle` (`self.K2_GetActorLocation`) (`.WorldLocation` (break `CPathNode` _output)) "TraceTypeQuery1"))
      (bind _output_get_2 (set `local.WasHit` _returnvalue))
      (if (not _output_get_2)
        (set `local.BestDot` (`local.CurrDot`))
        (`/Engine/EditorBlueprintResources/StandardMacros.IncrementInt` (`local.BestIndex`)
          (:`  `
            (if (>= (`local.BestIndex`) (- (`KismetArrayLibrary.Array_Length` (`self.PathBuffer`)) 2))
              (return (`local.BestIndex`))))))
      (else
        (return (`local.BestIndex`)))))
  (return (`local.BestIndex`)))

(fn `UserConstructionScript`)